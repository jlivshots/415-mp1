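; BP_Bullet is a projectile actor for InfiniteMatrix that flies along world X and destroys itself on impact or timeout.
; Construction adds the owning BP_Player's forward speed to the bullet's own speed.
; Tick moves it with a swept world offset and destroys it once it outlives MaxTime.
; Overlapping any static mesh component also destroys it.
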(event OnComponentBeginOverlap(bullet)
  (params (OverlappedComponent :type Primitive%20Component%20Object%20Reference) (OtherActor :type Actor%20Object%20Reference) (OtherComp :type Primitive%20Component%20Object%20Reference) (OtherBodyIndex :type Integer) (bFromSweep :type Boolean) (SweepResult :type Hit%20Result%20Structure%20%28by%20ref%29))
  (Utilities|Casting|CastToStaticMeshComponent OtherComp)
  (Actor|DestroyActor))

(event EventBeginPlay)

(event Collision|EventActorBeginOverlap
  (params (OtherActor :type Actor%20Object%20Reference)))

(event EventTick
  (params (DeltaSeconds :type Float%20%28single-precision%29))
  (Transformation|AddActorWorldOffset (Math|Vector|MakeVector (* DeltaSeconds (Variables|Default|GetForwardSpeed)) 0.0 0.0) true)
  (if (> (Actor|GetGameTimeSinceCreation) (Variables|Default|GetMaxTime))
    (Actor|DestroyActor)))

(fn ConstructionScript
  (bind _asbp_player (Utilities|Casting|CastToBP_Player (Components|GetOwner)))
  (Variables|Default|SetForwardSpeed (+ (Variables|Default|GetBulletSpeedOnly) (Variables|/Game/InfiniteMatrix/Blueprints/BP_Player.BP_Player_C|GetForwardSpeed _asbp_player))))